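; BP_PeopleLaunch is a person actor that gets knocked flying as a ragdoll by an attacker.
; Its Ragdoll event runs once, turning on mesh physics simulation and applying a fixed-strength impulse as a velocity change, directed away from the attacker with an upward bias.
; It then calls SetActorLocationAndRotation; BeginPlay, overlap and construction logic are empty.
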(event Custom|Ragdoll
  (params (Attacker :type Actor%20Object%20Reference))
  (Utilities|FlowControl|DoOnce false
    (:Completed
      (Physics|SetSimulatePhysics (Variables|Character|GetMesh) true)
      (Physics|AddImpulse (Variables|Character|GetMesh) (* (Math|Vector|Normalize (Utilities|Operators|Subtract (Transformation|GetActorLocation) (Transformation|GetActorLocation Attacker) "0.000000,0.000000,-50.000000")) 1.55e+04) "None" true)
      (Transformation|SetActorLocationAndRotation "0, 0, 0" "0, 0, 0"))))

(event EventBeginPlay)

(event Collision|EventActorBeginOverlap
  (params (OtherActor :type Actor%20Object%20Reference)))

(fn ConstructionScript)